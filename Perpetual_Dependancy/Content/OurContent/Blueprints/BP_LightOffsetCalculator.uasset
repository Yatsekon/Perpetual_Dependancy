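; BP_LightOffsetCalculator is a utility actor that computes each light's offset from the center of its room.
; On BeginPlay it casts each Test element to Room31, gets its cell center, subtracts the same-index GroupActorLight location and appends the result to Vector3Offset.
; Disconnected variants using GroupActorRoom locations or T7C0 room centers remain in the graph but never run.
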(event `self.ReceiveBeginPlay`
  ;[1 0.2681 0.5654] Calcule l'offset des lumières par rapport au centre pour bp spécifique
  (for (_array_element _array_index) (`self.Test`)
    (bind _asroom_31 (cast `/Game/OurContent/Blueprints/LevelPrefab/Room31` _array_element))
    (bind _wallcenter (`/Game/OurContent/Blueprints/LevelPrefab/BP_ParentRoom.DetermineCellCenter` _asroom_31))
    (`KismetArrayLibrary.Array_Add` (`self.Vector3Offset`) (- _wallcenter (`self.K2_GetActorLocation` (`|GetArrayItem` (`self.GroupActorLight`) _array_index))))))

(fn `UserConstructionScript`)