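; BP_Door is a room-exit door that acts when an actor overlaps its trigger box.
; A normal door asks the Room_Manager for the next room, passing its loop-door flag; if locked, it first consumes the player character's key or plays a locked sound.
; A secret door instead clears the player controller's addiction flag and starts the game outro once.
; SetMatSecretDoor swaps the door mesh to the antidote material.
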(event `self.ReceiveBeginPlay`
  (bind _returnvalue (`GameplayStatics.GetActorOfClass` "/Game/OurContent/Blueprints/Room_Manager.Room_Manager_C"))
  (set `self.RoomManager` _returnvalue))

(event `self.Box.OnComponentBeginOverlap`
  (params (OverlappedComponent :type "PrimitiveComponent Object Reference") (OtherActor :type "Actor Object Reference") (OtherComp :type "PrimitiveComponent Object Reference") (OtherBodyIndex :type Integer) (bFromSweep :type Boolean) (SweepResult :type "HitResult Structure (by ref)"))
  (if (not (`self.B_IsSecretDoor`))
    (bind _asbp_third_person_character (cast `/Game/ThirdPerson/Blueprints/BP_ThirdPersonCharacter` OtherActor))
    (if (`self.NeedKey`)
      (if (`/Game/ThirdPerson/Blueprints/BP_ThirdPersonCharacter.B_HasKey` _asbp_third_person_character)
        (`/Engine/EditorBlueprintResources/StandardMacros.DoOnce` false
          (:`Completed`
            (set `/Game/ThirdPerson/Blueprints/BP_ThirdPersonCharacter.B_HasKey` false _asbp_third_person_character)
            (bind _asbp_player_controller (cast `/Game/OurContent/Blueprints/BP_PlayerController` (`GameplayStatics.GetPlayerController` 0))
              (:`then`
                (`/Game/OurContent/Blueprints/BP_PlayerController.DisableKey` _asbp_player_controller))
              (:`CastFailed`
                _))
            (`/Game/OurContent/Blueprints/Room_Manager.NewNextRoom` (`self.RoomManager`) (`self.B_IsLoopDoor`))))
        (else
          (`GameplayStatics.PlaySound2D` "/Game/OurContent/Sounds/Environnement/Door_Locked_-_01_Cue.Door_Locked_-_01_Cue" 1.0 1.0 0.0 null null)))
      (else
        (`/Game/OurContent/Blueprints/Room_Manager.NewNextRoom` (`self.RoomManager`) (`self.B_IsLoopDoor`))))
    (else
      (bind _asbp_player_controller_2 (cast `/Game/OurContent/Blueprints/BP_PlayerController` (`GameplayStatics.GetPlayerController` 0)))
      (`/Engine/EditorBlueprintResources/StandardMacros.DoOnce` false
        (:`Completed`
          (set `/Game/OurContent/Blueprints/BP_PlayerController.B_IsAddictionOn` false _asbp_player_controller_2)
          (`/Game/OurContent/Blueprints/BP_PlayerController.OutroOfTheGame` _asbp_player_controller_2))))))

(fn `SetMatSecretDoor`
  (`PrimitiveComponent.SetMaterial` (`self.Door`) 0 "/Game/Game_art/Meshes/props/Door_Antidote.Door_Antidote"))

(fn `UserConstructionScript`)