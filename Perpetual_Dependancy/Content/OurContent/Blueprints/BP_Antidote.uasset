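; BP_Antidote is a one-use drinkable pickup that resets the player's addiction and spawns a secret door in the current room.
; Interaction drives the player controller's HUD buff, text and music switch, swaps to the open-bottle mesh and triggers any parent room event.
; Until drunk, its name label yaws toward the player and shows briefly on ReadName, while box overlap toggles an outline overlay material.
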(event `/Game/OurContent/Blueprints/Other/I_Interact.PlayerInteraction`
  (params (Interactor :type "Character Object Reference"))
  (bind _parentroom_event_ (`self.ParentRoom(Event)`))
  (bind _asbp_player_controller (cast `/Game/OurContent/Blueprints/BP_PlayerController` (`GameplayStatics.GetPlayerController` 0)))
  (`/Engine/EditorBlueprintResources/StandardMacros.DoOnce` false
    (:`Completed`
      (`/Game/OurContent/Blueprints/LevelPrefab/BP_ParentRoom.SpawnSecretDoor` (`/Game/OurContent/Blueprints/BP_PlayerController.BP_CurrentRoom` _asbp_player_controller))
      (`/Game/OurContent/Blueprints/BP_PlayerController.ResetAddiction` _asbp_player_controller)
      (`/Game/OurContent/Widgets/WG_Hud.PlayAntidoteBuff` (`/Game/OurContent/Blueprints/BP_PlayerController.WG_HUD` _asbp_player_controller))
      (`/Game/OurContent/Blueprints/BP_PlayerController.StopAllSound` _asbp_player_controller)
      (`/Game/OurContent/Blueprints/BP_PlayerController.DisplayTextAntidote` _asbp_player_controller)
      (`StaticMeshComponent.SetStaticMesh` (`self.Model`) "/Game/Game_art/Meshes/props/MSH_popo_antidote_open.MSH_popo_antidote_open")
      (`GameplayStatics.PlaySound2D` "/Game/OurContent/Sounds/Items/Antidote_Drink_-_03_Cue.Antidote_Drink_-_03_Cue" 1.0 1.0 0.0 null null)
      (`/Game/OurContent/Blueprints/BP_PlayerController.Switch Music` _asbp_player_controller "/Game/OurContent/Sounds/Music/Roomtone_02_-_01_Cue.Roomtone_02_-_01_Cue")
      (set `self.B_IsDrunk` true)
      (`SceneComponent.SetVisibility` (`self.TextRender`) false false)
      (`MeshComponent.SetOverlayMaterial` (`self.Model`) null)
      (`/Engine/EditorBlueprintResources/StandardMacros.IsValid` _parentroom_event_
        (:`Is Valid`
          (`/Game/OurContent/Blueprints/LevelPrefab/BP_ParentRoom.Display Event` _parentroom_event_ (`/Game/OurContent/Blueprints/LevelPrefab/BP_ParentRoom.SC_ObjEventToSpawn` _parentroom_event_)))))))

(event `self.ReceiveTick`
  (params (DeltaSeconds :type "Float (single-precision)"))
  (bind (_returnvalue_roll _returnvalue_pitch) (`KismetMathLibrary.BreakRotator` (`SceneComponent.K2_GetComponentRotation` (`self.TextRender`))))
  (bind (_returnvalue_roll_2 _returnvalue_pitch_2 _returnvalue_yaw) (`KismetMathLibrary.BreakRotator` (`KismetMathLibrary.FindLookAtRotation` (`SceneComponent.K2_GetComponentLocation` (`self.TextRender`)) (`self.K2_GetActorLocation` (`GameplayStatics.GetPlayerPawn` 0)))))
  (if (not (`self.B_IsDrunk`))
    (`SceneComponent.K2_SetWorldRotation` (`self.TextRender`) (`KismetMathLibrary.MakeRotator` _returnvalue_roll _returnvalue_pitch _returnvalue_yaw) false false)
    (if (not (`self.B_IsReadable`))
      (`SceneComponent.SetVisibility` (`self.TextRender`) false false))))

(event `/Game/OurContent/Blueprints/Other/I_DisplayName.Read Name`
  (if (not (`self.B_IsDrunk`))
    (set `self.B_IsReadable` true)
    (`/Engine/EditorBlueprintResources/StandardMacros.DoOnce` false :!label _label
      (:`Completed`
        (`SceneComponent.SetVisibility` (`self.TextRender`) true false)
        (`KismetSystemLibrary.Delay` 0.5)
        (set `self.B_IsReadable` false)
        (goto _label :!via `Reset`)))))

(event `self.Box.OnComponentBeginOverlap`
  (params (OverlappedComponent :type "PrimitiveComponent Object Reference") (OtherActor :type "Actor Object Reference") (OtherComp :type "PrimitiveComponent Object Reference") (OtherBodyIndex :type Integer) (bFromSweep :type Boolean) (SweepResult :type "HitResult Structure (by ref)"))
  (if (== OtherActor (`GameplayStatics.GetPlayerPawn` 0))
    (if (not (`self.B_IsDrunk`))
      (`MeshComponent.SetOverlayMaterial` (`self.Model`) "/Game/OurContent/Material/Outline/Mi_Outline_Antidote.Mi_Outline_Antidote"))))

(event `self.Box.OnComponentEndOverlap`
  (params (OverlappedComponent :type "PrimitiveComponent Object Reference") (OtherActor :type "Actor Object Reference") (OtherComp :type "PrimitiveComponent Object Reference") (OtherBodyIndex :type Integer))
  (if (== OtherActor (`GameplayStatics.GetPlayerPawn` 0))
    (`MeshComponent.SetOverlayMaterial` (`self.Model`) null)))

(fn `UserConstructionScript`)