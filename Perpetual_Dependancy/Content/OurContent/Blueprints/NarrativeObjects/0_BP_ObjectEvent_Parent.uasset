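; Parent Blueprint for narrative object events that trigger a hallucination and dialogue when the player character enters the box.
; After a configurable delay, it fires once, adding a hallucination post-process to the character and swapping Structure's child materials to a glitch material.
; It sends the player controller either flip-flop dialogue or a random narrative text.
; Only the random-text path then removes the effect, plays a disappear sound and destroys the actor.
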(event `self.ReceiveBeginPlay`
  (set `self.InitMaterial` (`MeshComponent.GetMaterials` (`self.StaticMesh`))))

(event `self.Box.OnComponentBeginOverlap`
  (params (OverlappedComponent :type "PrimitiveComponent Object Reference") (OtherActor :type "Actor Object Reference") (OtherComp :type "PrimitiveComponent Object Reference") (OtherBodyIndex :type Integer) (bFromSweep :type Boolean) (SweepResult :type "HitResult Structure (by ref)"))
  (bind _int_textnumber (`self.Int_TextNumber`))
  (bind _f_dialoguedisplaysuppl (`self.F_DialogueDisplaySuppl`))
  (`KismetSystemLibrary.Delay` (`self.F_WaitingTime`))
  (bind _asbp_third_person_character (cast `/Game/ThirdPerson/Blueprints/BP_ThirdPersonCharacter` OtherActor))
  (`/Engine/EditorBlueprintResources/StandardMacros.DoOnce` false
    (:`Completed`
      (`/Game/ThirdPerson/Blueprints/BP_ThirdPersonCharacter.AddPostProcessEffect` _asbp_third_person_character "/Game/Game_art/Post_process/hallu/Hallucination_Inst_3.Hallucination_Inst_3")
      (for _array_element (`SceneComponent.GetChildrenComponents` (`self.Structure`) false)
        (bind _asprimitive_component (cast `PrimitiveComponent` _array_element)
          (:`then`
            _)
          (:`CastFailed`
            _))
        (for (_ _array_index) (`self.InitMaterial`)
          (`PrimitiveComponent.SetMaterial` _asprimitive_component _array_index (`self.Glitch_Material`))))
      (bind _asbp_player_controller (cast `/Game/OurContent/Blueprints/BP_PlayerController` (`GameplayStatics.GetPlayerController` 0)))
      (if (`self.IsFlipFlopSystem`)
        (`/Game/OurContent/Blueprints/BP_PlayerController.Set Dialogue FlipFlopSystem` _asbp_player_controller _int_textnumber _f_dialoguedisplaysuppl)
        (else
          (`/Game/OurContent/Blueprints/BP_PlayerController.SetNarrativeTexts` _asbp_player_controller (`KismetArrayLibrary.Array_Random` _int_textnumber) _f_dialoguedisplaysuppl 0.0)
          (`KismetSystemLibrary.Delay` (`self.F_effectDuration`))
          (`/Game/ThirdPerson/Blueprints/BP_ThirdPersonCharacter.RemovePostProcessEffect` _asbp_third_person_character "/Game/Game_art/Post_process/hallu/Hallucination_Inst_3.Hallucination_Inst_3")
          (`GameplayStatics.SpawnSoundAtLocation` "/Game/OurContent/Sounds/Items/SFX_Object_Disappear_01_Cue.SFX_Object_Disappear_01_Cue" (`self.K2_GetActorLocation` self) (struct) 1.0 1.0 0.0 null null)
          (`KismetSystemLibrary.Delay` 0.5)
          (`self.K2_DestroyActor`))))))

(fn `UserConstructionScript`)