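; Drinkable poison glass pickup with a localized name label that yaws toward the player.
; A box overlap toggles an outline overlay and tutorial prompt, while ReadName briefly reveals the label.
; PlayerInteraction queues the effect on the character by room count, or applies it immediately, extending it if already active.
; Drinking also raises controller addiction, plays a sound, swaps the mesh and disables further interaction.
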(event `self.ReceiveBeginPlay`
  (bind _textrender (`self.TextRender`))
  (set `self.S_Poison_Stats` (make `/Game/OurContent/Blueprints/Other/S_PoisonStats` (`self.E_Effect`) (`self.Int_EffectDuration`) (`self.Int_EffectDelay`) (`self.Int_PoisonPower`) (`self.F_AddictionBoost`) (`self.F_SpeedMultiplier`) (`self.GravityScaleModifier`) (`self.JumpVelocityModifier`) (`self.Int_MinStumble`) (`self.Int_MaxStumble`) (`self.F_MinDelayStumble`) (`self.F_MaxDelayStumble`)))
  (bind _asmy_game_instance (cast `/Game/OurContent/Blueprints/MyGameInstance` (`GameplayStatics.GetGameInstance`))
    (:`then`
      (switch `int` (`/Game/OurContent/Blueprints/MyGameInstance.Int_Localization` _asmy_game_instance)
        (:`0`
          (`TextRenderComponent.K2_SetText` _textrender (`self.Name`) :!label _label))
        (:`1`
          (`TextRenderComponent.K2_SetText` _textrender (`self.Fr_Name`)))))
    (:`CastFailed`
      (goto _label)))
  (`StaticMeshComponent.SetStaticMesh` (`self.Model`) (`|GetArrayItem` (`self.Props_Poison`)))
  (`TextRenderComponent.SetTextRenderColor` (`self.TextRender`) (`self.PoisonTextColor`)))

(event `self.ReceiveTick`
  (params (DeltaSeconds :type "Float (single-precision)"))
  (bind (_returnvalue_roll _returnvalue_pitch) (`KismetMathLibrary.BreakRotator` (`SceneComponent.K2_GetComponentRotation` (`self.TextRender`))))
  (bind (_returnvalue_roll_2 _returnvalue_pitch_2 _returnvalue_yaw) (`KismetMathLibrary.BreakRotator` (`KismetMathLibrary.FindLookAtRotation` (`SceneComponent.K2_GetComponentLocation` (`self.TextRender`)) (`self.K2_GetActorLocation` (`GameplayStatics.GetPlayerPawn` 0)))))
  (if (not (`self.B_IsDrunk`))
    (`SceneComponent.K2_SetWorldRotation` (`self.TextRender`) (`KismetMathLibrary.MakeRotator` _returnvalue_roll _returnvalue_pitch _returnvalue_yaw) false false)
    (if (not (`self.B_IsReadable`))
      (`SceneComponent.SetVisibility` (`self.TextRender`) false false))))

(event `/Game/OurContent/Blueprints/Other/I_Interact.PlayerInteraction`
  (params (Interactor :type "Character Object Reference"))
  (bind _int_effectdelay (`self.Int_EffectDelay`))
  (bind _as_bp_player_controller (`self.As BP Player Controller`))
  (bind _as_bp_player_controller_2 (`self.As BP Player Controller`))
  (bind _as_bp_third_person_character (`self.As BP Third Person Character`))
  (bind _as_bp_third_person_character_2 (`self.As BP Third Person Character`))
  (bind _as_bp_third_person_character_3 (`self.As BP Third Person Character`))
  (bind _returnvalue (`KismetArrayLibrary.Array_Find` (`/Game/ThirdPerson/Blueprints/BP_ThirdPersonCharacter.PoisonEffectActive` _as_bp_third_person_character) (`self.E_Effect`)))
  (bind _asbp_third_person_character (cast `/Game/ThirdPerson/Blueprints/BP_ThirdPersonCharacter` Interactor))
  (set `self.As BP Third Person Character` _asbp_third_person_character)
  (bind _asbp_player_controller (cast `/Game/OurContent/Blueprints/BP_PlayerController` (`GameplayStatics.GetPlayerController` 0)))
  (set `self.As BP Player Controller` _asbp_player_controller)
  (if (> _int_effectdelay 0)
    (set `self.Int_EffectDelay` (+ _int_effectdelay (`/Game/OurContent/Blueprints/BP_PlayerController.RoomCount` (`self.As BP Player Controller`))))
    (`KismetArrayLibrary.Array_Add` (`/Game/ThirdPerson/Blueprints/BP_ThirdPersonCharacter.PoisonDelayStats` _as_bp_third_person_character_3) (`self.S_Poison_Stats`))
    (`KismetArrayLibrary.Array_Add` (`/Game/ThirdPerson/Blueprints/BP_ThirdPersonCharacter.PoisonDelayRemaning` _as_bp_third_person_character_3) (make `/Game/OurContent/Blueprints/Other/S_PoisonDelay` (`self.E_Effect`) (`self.Int_EffectDelay`)))
    (elif (== _returnvalue -1)
      (`KismetArrayLibrary.Array_Add` (`/Game/ThirdPerson/Blueprints/BP_ThirdPersonCharacter.PoisonTurnRemaining` _as_bp_third_person_character_2) (+ (`/Game/OurContent/Blueprints/BP_PlayerController.RoomCount` (`self.As BP Player Controller`)) (`self.Int_EffectDuration`)))
      (`KismetArrayLibrary.Array_Add` (`/Game/ThirdPerson/Blueprints/BP_ThirdPersonCharacter.PoisonEffectActive` _as_bp_third_person_character_2) (`self.E_Effect`))
      (`/Game/ThirdPerson/Blueprints/BP_ThirdPersonCharacter.SwitchPoisonEffect` (`self.As BP Third Person Character`) (`self.S_Poison_Stats`))
      (else
        (`KismetArrayLibrary.Array_Set` (`/Game/ThirdPerson/Blueprints/BP_ThirdPersonCharacter.PoisonTurnRemaining` _as_bp_third_person_character_2) _returnvalue (+ (`|GetArrayItem` (`/Game/ThirdPerson/Blueprints/BP_ThirdPersonCharacter.PoisonTurnRemaining` _as_bp_third_person_character) _returnvalue) (`self.Int_EffectDuration`)) true))))
  (`KismetSystemLibrary.PrintString` "" true true (struct :`G` 0.66 :`B` 1.0 :`A` 1.0) 0.0)
  (set `/Game/OurContent/Blueprints/BP_PlayerController.F_AddictionCurrValue` (+ (* (`/Game/OurContent/Blueprints/BP_PlayerController.F_CurrentPoisonMultiplicateur` _as_bp_player_controller_2) (`self.Int_PoisonPower`)) (`/Game/OurContent/Blueprints/BP_PlayerController.F_AddictionCurrValue` _as_bp_player_controller_2)) _as_bp_player_controller_2)
  (`ActorComponent.K2_DestroyComponent` (`self.Box`))
  (`/Game/OurContent/Blueprints/BP_PlayerController.IncreaseAddiction` _as_bp_player_controller 1)
  (if (== (`/Game/OurContent/Blueprints/BP_PlayerController.Int_BoucleCount` _as_bp_player_controller) 0)
    (`/Game/OurContent/Blueprints/BP_PlayerController.DisplayTextPoison` _as_bp_player_controller))
  (bind _returnvalue_2 (`GameplayStatics.SpawnSound2D` (`self.Drink_Sound`) 1.0 1.0 0.0 null))
  (`/Game/OurContent/Blueprints/BP_PlayerController.ManageSoundEffect` _as_bp_player_controller _returnvalue_2)
  (`StaticMeshComponent.SetStaticMesh` (`self.Model`) (`|GetArrayItem` (`self.Props_Poison`) 1))
  (`SceneComponent.SetVisibility` (`self.TextRender`) false false)
  (`MeshComponent.SetOverlayMaterial` (`self.Model`) null)
  (`PrimitiveComponent.SetCollisionEnabled` (`self.Model`) "NoCollision")
  (set `self.B_IsDrunk` true)
  (`/Game/ThirdPerson/Blueprints/BP_ThirdPersonCharacter.SetTutoInteract` (`self.As BP Third Person Character`) true false true))

(event `/Game/OurContent/Blueprints/Other/I_DisplayName.Read Name`
  (bind _textrender (`self.TextRender`))
  (bind _asbp_third_person_character (cast `/Game/ThirdPerson/Blueprints/BP_ThirdPersonCharacter` (`GameplayStatics.GetPlayerPawn` 0))
    (:`then`
      (if (not (`/Game/ThirdPerson/Blueprints/BP_ThirdPersonCharacter.B_Stop_Display_Name` _asbp_third_person_character))
        (if (not (`self.B_IsDrunk`)) :!label _label_2
          (set `self.B_IsReadable` true)
          (`/Engine/EditorBlueprintResources/StandardMacros.DoOnce` false :!label _label_3
            (:`Completed`
              (`SceneComponent.SetVisibility` _textrender true false)
              (`KismetSystemLibrary.PrintString` (`KismetTextLibrary.Conv_TextToString` (`TextRenderComponent.Text` _textrender)))
              (`KismetSystemLibrary.PrintString` (`KismetStringLibrary.Concat_StrStr` "Is Poison Name Visible ? " (`KismetStringLibrary.Conv_BoolToString` (`SceneComponent.bVisible` _textrender))))
              (`KismetSystemLibrary.Delay` 0.5)
              (set `self.B_IsReadable` false)
              (goto _label_3 :!via `Reset`))))))
    (:`CastFailed`
      (goto _label_2))))

(event `self.Box.OnComponentBeginOverlap`
  (params (OverlappedComponent :type "PrimitiveComponent Object Reference") (OtherActor :type "Actor Object Reference") (OtherComp :type "PrimitiveComponent Object Reference") (OtherBodyIndex :type Integer) (bFromSweep :type Boolean) (SweepResult :type "HitResult Structure (by ref)"))
  (bind _returnvalue (`GameplayStatics.GetPlayerPawn` 0))
  (if (== OtherActor _returnvalue)
    (bind _asbp_third_person_character (cast `/Game/ThirdPerson/Blueprints/BP_ThirdPersonCharacter` _returnvalue)
      (:`then`
        (if (not (`/Game/ThirdPerson/Blueprints/BP_ThirdPersonCharacter.B_StopDisplay_GreenTexture` _asbp_third_person_character))
          (if (not (`self.B_IsDrunk`)) :!label _label_4
            (`MeshComponent.SetOverlayMaterial` (`self.Model`) "/Game/OurContent/Material/Outline/Mi_OutlinePoison.Mi_OutlinePoison")
            (bind _asbp_third_person_character_2 (cast `/Game/ThirdPerson/Blueprints/BP_ThirdPersonCharacter` OtherActor))
            (`/Game/ThirdPerson/Blueprints/BP_ThirdPersonCharacter.SetTutoInteract` _asbp_third_person_character_2 true true false))))
      (:`CastFailed`
        (goto _label_4)))))

(event `self.Box.OnComponentEndOverlap`
  (params (OverlappedComponent :type "PrimitiveComponent Object Reference") (OtherActor :type "Actor Object Reference") (OtherComp :type "PrimitiveComponent Object Reference") (OtherBodyIndex :type Integer))
  (if (== OtherActor (`GameplayStatics.GetPlayerPawn` 0))
    (`MeshComponent.SetOverlayMaterial` (`self.Model`) null)
    (bind _asbp_third_person_character (cast `/Game/ThirdPerson/Blueprints/BP_ThirdPersonCharacter` OtherActor))
    (`/Game/ThirdPerson/Blueprints/BP_ThirdPersonCharacter.SetTutoInteract` _asbp_third_person_character true false false)))

(fn `UserConstructionScript`)