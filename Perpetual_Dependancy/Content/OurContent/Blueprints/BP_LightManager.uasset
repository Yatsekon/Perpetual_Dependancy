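; Light manager that relocates pre-placed, per-room groups of lights to the active room's position.
; On BeginPlay it caches each parent actor's attached actors and their offsets from that room's center actor.
; SetupLightning moves the previous room's group to a holding location, except on first use, then moves the new room's group in.
; Each move repositions the center actor using a per-room offset, then rebuilds light positions from cached offsets.
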(event `GroupactorRef`
  ;[0.01042 0.01042 0.01042] Archive
  (for _array_element (`self.GroupeActor`)
    (`KismetArrayLibrary.Array_Add` (`self.GA Location`) (`self.K2_GetActorLocation` _array_element))))

(event `self.ReceiveBeginPlay`
  (for (_array_element _array_index) (`self.ParentActor`)
    (set `self.ParentActor Index` _array_index)
    (bind _outactors (`self.GetAttachedActors` _array_element true false))
    ;[0.3854 0.3492 0.06223] Calcule la distance entre les lights et leur centre
    (for _array_element_2 _outactors
      (`KismetArrayLibrary.Array_Add` (`self.Ar_LightRelativeLocation`) (- (`self.K2_GetActorLocation` _array_element_2) (`self.K2_GetActorLocation` (`|GetArrayItem` (`self.CenterActor`) (`self.ParentActor Index`))))))
    (`KismetArrayLibrary.Array_Add` (`self.Ar_ChildrenActors`) (make `/Game/OurContent/Blueprints/Other/S_LightArray` _outactors (`self.Ar_LightRelativeLocation`)))
    (`KismetArrayLibrary.Array_Clear` (`self.Ar_LightRelativeLocation`))))

(event `SetupLightning`
  (params (RoomTransform :type "Vector Structure") (RoomNumber :type Integer) (LastRoom :type Integer))
  (bind _output_ar_lightchildren (break `/Game/OurContent/Blueprints/Other/S_LightArray` (`|GetArrayItem` (`self.Ar_ChildrenActors`) LastRoom)))
  (bind _output_ar_lightchildren_2 (break `/Game/OurContent/Blueprints/Other/S_LightArray` (`|GetArrayItem` (`self.Ar_ChildrenActors`) (`self.Room Number`))))
  ;[0.3854 0.3492 0.06223] Setup Light
  (set `self.Room Number` RoomNumber)
  (if (not (`self.B_FirstRoom`))
    (`self.ModifyLightsLocation` (`self.V_NewLocationForPrecedentsLights`) _output_ar_lightchildren LastRoom))
  (`self.ModifyLightsLocation` RoomTransform _output_ar_lightchildren_2 (`self.Room Number`))
  (set `self.B_FirstRoom` false))

(event `ModifyLightsLocation`
  (params (NewLightPos :type "Vector Structure") (Lights :type "Array of Actor Object Reference") (CorrespondingRoom :type Integer))
  (bind (_output_ar_lightchildren _output_ar_relativelocation) (break `/Game/OurContent/Blueprints/Other/S_LightArray` (`|GetArrayItem` (`self.Ar_ChildrenActors`) (`self.CorrespondingRoom`))))
  (bind _output_get (set `self.CorrespondingRoom` CorrespondingRoom))
  (`self.K2_SetActorLocation` (`|GetArrayItem` (`self.CenterActor`) _output_get) (- NewLightPos (`|GetArrayItem` (`self.Ar_LocationOffSet`) _output_get)) false false)
  ;[0.3854 0.3492 0.06223] Replace les lumières par rapport à leur distance relative avec l'actor
  (for (_array_element _array_index) Lights
    (bind (_returnvalue_x _returnvalue_y _returnvalue_z) (`KismetMathLibrary.BreakVector` (+ (`|GetArrayItem` _output_ar_relativelocation _array_index) (`self.K2_GetActorLocation` (`|GetArrayItem` (`self.CenterActor`) (`self.CorrespondingRoom`))))))
    (`self.K2_SetActorLocation` _array_element (`KismetMathLibrary.MakeVector` _returnvalue_x _returnvalue_y _returnvalue_z) false false)))

(fn `UserConstructionScript`)