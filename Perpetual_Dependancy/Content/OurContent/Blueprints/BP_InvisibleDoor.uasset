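; BP_InvisibleDoor is a door that starts invisible and can be revealed through its Display event.
; On BeginPlay it caches each material of the Door component in GetInitMaterials, then swaps that slot to M_Alpha0.
; Display writes the cached materials back by slot index; nothing in this Blueprint calls it, and only materials are changed, with no collision or visibility toggles.
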(event `self.ReceiveBeginPlay`
  (`parent.ReceiveBeginPlay`)
  (for (_array_element _array_index) (`MeshComponent.GetMaterials` (`self.Door`))
    (`KismetArrayLibrary.Array_Add` (`self.GetInitMaterials`) _array_element)
    (`PrimitiveComponent.SetMaterial` (`self.Door`) _array_index "/Game/OurContent/Material/M_Alpha0.M_Alpha0")))

(event `Display`
  (for (_array_element _array_index) (`self.GetInitMaterials`)
    (`PrimitiveComponent.SetMaterial` (`self.Door`) _array_index _array_element)))

(fn `UserConstructionScript`
  (`parent.UserConstructionScript`))