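; BP_Spawner is a spawn point that places a poison or an antidote at its Sphere component's transform.
; Poisons are either spawned from a given class, which is passed to the controller's PoisonGenerator unless flagged BCantBeRdmPoison, or obtained through the controller's PoisonRdm.
; SpawnAntidote creates and returns a BP_Antidote and sets a flag.
; That flag tells OnDestroyCustom whether to destroy the stored antidote or poison.
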(event `self.ReceiveBeginPlay`)

(event `PoisonToSpawn`
  (params (PoisonToSpawn :type "/Game/OurContent/Blueprints/PoisonList/1Bp_Poison_Glasses Class Reference") (BP_PController :type "/Game/OurContent/Blueprints/BP_PlayerController Object Reference"))
  (bind _returnvalue (`|SpawnActorFromClass` PoisonToSpawn (`SceneComponent.K2_GetComponentToWorld` (`self.Sphere`)) "Undefined" "MultiplyWithRoot" null null))
  (bind _output_get (set `self.BP_Poison` _returnvalue))
  (if (not (`/Game/OurContent/Blueprints/PoisonList/1Bp_Poison_Glasses.b_CantBeRdmPoison` _output_get))
    (`/Game/OurContent/Blueprints/BP_PlayerController.Poison Generator` BP_PController (`GameplayStatics.GetObjectClass` _output_get))))

(event `OnDestroyCustom`
  (if (not (`self.GetAntidoteSpawned`))
    (`self.K2_DestroyActor` (`self.BP_Poison`))
    (else
      (`self.K2_DestroyActor` (`self.BP_Antidote`)))))

(event `RandomPoisonSpawn`
  (params (BP_PController :type "/Game/OurContent/Blueprints/BP_PlayerController Object Reference"))
  (bind _bp_poison (`/Game/OurContent/Blueprints/BP_PlayerController.PoisonRdm` BP_PController (`SceneComponent.K2_GetComponentToWorld` (`self.Sphere`))))
  (set `self.BP_Poison` _bp_poison))

(fn `SpawnAntidote`
  (returns (AntidoteSpawned :type "/Game/OurContent/Blueprints/BP_Antidote Object Reference"))
  (bind _returnvalue (`|SpawnActorFromClass` "/Game/OurContent/Blueprints/BP_Antidote.BP_Antidote_C" (`SceneComponent.K2_GetComponentToWorld` (`self.Sphere`)) "Undefined" "MultiplyWithRoot" null null))
  (bind _output_get (set `self.BP_Antidote` _returnvalue))
  (set `self.GetAntidoteSpawned` true)
  (return _output_get))

(fn `UserConstructionScript`)