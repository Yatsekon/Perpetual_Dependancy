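; Checkpoint actor that saves the player's progress as the current room number and loop count in MyGameInstance.
; When the third-person character enters its box, it saves once, provided Room_Manager's room is beyond the last checkpoint or the loop count has increased.
; Feedback is a timeline-driven point light, followed by a sound chosen by loop count.
; A separate event swaps the material on its three meshes.
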(event `self.ReceiveBeginPlay`
  (bind _returnvalue (`GameplayStatics.GetActorOfClass` "/Game/OurContent/Blueprints/Room_Manager.Room_Manager_C"))
  (set `self.RoomManagerRef` _returnvalue))

(event `self.Box.OnComponentBeginOverlap`
  (params (OverlappedComponent :type "PrimitiveComponent Object Reference") (OtherActor :type "Actor Object Reference") (OtherComp :type "PrimitiveComponent Object Reference") (OtherBodyIndex :type Integer) (bFromSweep :type Boolean) (SweepResult :type "HitResult Structure (by ref)"))
  (bind _returnvalue (`SceneComponent.K2_GetComponentLocation` (`self.StaticMesh3`)))
  (cast `/Game/ThirdPerson/Blueprints/BP_ThirdPersonCharacter` OtherActor)
  (bind _asmy_game_instance (cast `/Game/OurContent/Blueprints/MyGameInstance` (`GameplayStatics.GetGameInstance`)))
  (if (or (> (`/Game/OurContent/Blueprints/Room_Manager.RoomNumber` (`self.RoomManagerRef`)) (`/Game/OurContent/Blueprints/MyGameInstance.LastCheckpoint` _asmy_game_instance)) (> (`/Game/OurContent/Blueprints/MyGameInstance.LoopsCount` _asmy_game_instance) (`/Game/OurContent/Blueprints/MyGameInstance.LastCheckpointLoop` _asmy_game_instance)))
    (`/Engine/EditorBlueprintResources/StandardMacros.DoOnce` false
      (:`Completed`
        (set `/Game/OurContent/Blueprints/MyGameInstance.LastCheckpoint` (`/Game/OurContent/Blueprints/Room_Manager.RoomNumber` (`self.RoomManagerRef`)) _asmy_game_instance)
        (set `/Game/OurContent/Blueprints/MyGameInstance.LastCheckpointLoop` (`/Game/OurContent/Blueprints/MyGameInstance.LoopsCount` _asmy_game_instance) _asmy_game_instance)
        ;[0.0625 0.0625 0.0625] Feedback
        (bind (_direction _newtrack_0) (`Timeline|LightOn` :!via `PlayFromStart`)
          (:`Update`
            (`LightComponent.SetIntensity` (`self.PointLight`) _newtrack_0))
          (:`Finished`
            (switch `int` (`/Game/OurContent/Blueprints/MyGameInstance.LoopsCount` _asmy_game_instance)
              (:`Default`
                (`GameplayStatics.PlaySoundAtLocation` "/Game/OurContent/Sounds/Environnement/Checkpoint_03_Cue.Checkpoint_03_Cue" _returnvalue (struct) 1.0 1.0 0.0 null null null null :!label _label))
              (:`0`
                (`GameplayStatics.PlaySoundAtLocation` "/Game/OurContent/Sounds/Environnement/Checkpoint_01_Cue.Checkpoint_01_Cue" _returnvalue (struct) 1.0 1.0 0.0 null null null null))
              (:`1`
                (`GameplayStatics.PlaySoundAtLocation` "/Game/OurContent/Sounds/Environnement/Checkpoint_02_Cue.Checkpoint_02_Cue" _returnvalue (struct) 1.0 1.0 0.0 null null null null))
              (:`2`
                (goto _label)))))))))

(event `ModifyComponentsMaterial`
  (params (MatToChange :type "MaterialInterface Object Reference"))
  (`PrimitiveComponent.SetMaterial` (`self.StaticMesh1`) 0 MatToChange)
  (`PrimitiveComponent.SetMaterial` (`self.StaticMesh2`) 0 MatToChange)
  (`PrimitiveComponent.SetMaterial` (`self.StaticMesh3`) 0 MatToChange))

(fn `UserConstructionScript`)