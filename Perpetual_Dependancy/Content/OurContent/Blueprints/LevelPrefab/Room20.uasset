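; Room20 is a level prefab room that shows a reading sheet event on a specific game loop.
; On BeginPlay it hides the sheet and a mesh, waits briefly, then runs antidote-count and event-destroy checks.
; If the player controller's loop count equals the required one, it reveals both and configures the child sheet actor's number and main-character commentary line.
; Otherwise it destroys the mesh component.
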(event `self.ReceiveBeginPlay`
  (`parent.ReceiveBeginPlay`)
  (`SceneComponent.SetVisibility` (`self.ReadingSheet`) false false)
  (`SceneComponent.SetVisibility` (`self.StaticMesh6`) false false)
  (`KismetSystemLibrary.Delay` 0.1)
  (`self.DoNotCountAntidote` false)
  (`self.CheckEventDestroy` (`self.ReadingSheet`))
  (if (== (`/Game/OurContent/Blueprints/BP_PlayerController.Int_BoucleCount` (`self.BP_PlayerController`)) (`self.boucleEventNeeded`))
    (`SceneComponent.SetVisibility` (`self.ReadingSheet`) true false)
    (`SceneComponent.SetVisibility` (`self.StaticMesh6`) true false)
    (bind _asbp_reading_sheet (cast `/Game/OurContent/Blueprints/Bp_ReadingSheet` (`ChildActorComponent.ChildActor` (`self.ReadingSheet`))))
    (set `/Game/OurContent/Blueprints/Bp_ReadingSheet.SheetNumber` 1 _asbp_reading_sheet)
    (set `/Game/OurContent/Blueprints/Bp_ReadingSheet.is_MC_Commentaring` true _asbp_reading_sheet)
    (set `/Game/OurContent/Blueprints/Bp_ReadingSheet.Int_commentaringNumber` 19 _asbp_reading_sheet)
    (else
      (`ActorComponent.K2_DestroyComponent` (`self.StaticMesh6`)))))

(fn `UserConstructionScript`
  (`parent.UserConstructionScript`))