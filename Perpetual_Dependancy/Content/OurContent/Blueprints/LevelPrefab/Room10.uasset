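; Room10 is a level prefab Blueprint for a looping narrative game that adapts its contents to the current loop.
; After a short BeginPlay delay, it triggers narrative text and pad music on the first loop, then runs destroy checks on its object and sheet event actors.
; When the controller's loop count matches the required value, it swaps meshes by destroying one and configures the readable sheet for character commentary.
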(event `self.ReceiveBeginPlay`
  (`parent.ReceiveBeginPlay`)
  (`KismetSystemLibrary.Delay` 0.1)
  (`self.NarrativeText`)
  (`self.CheckEventDestroy` (`self.ObjEvent`))
  (`self.CheckEventDestroy` (`self.SheetEvent`))
  (if (== (`/Game/OurContent/Blueprints/BP_PlayerController.Int_BoucleCount` (`self.BP_PlayerController`)) (`self.boucleEventNeeded`))
    (`ActorComponent.K2_DestroyComponent` (`self.StaticMesh`))
    (bind _asbp_reading_sheet (cast `/Game/OurContent/Blueprints/Bp_ReadingSheet` (`ChildActorComponent.ChildActor` (`self.SheetEvent`))))
    (set `/Game/OurContent/Blueprints/Bp_ReadingSheet.SheetNumber` 0 _asbp_reading_sheet)
    (set `/Game/OurContent/Blueprints/Bp_ReadingSheet.is_MC_Commentaring` true _asbp_reading_sheet)
    (set `/Game/OurContent/Blueprints/Bp_ReadingSheet.Int_commentaringNumber` 11 _asbp_reading_sheet)
    (else
      (`ActorComponent.K2_DestroyComponent` (`self.StaticMesh8`)))))

(event `NarrativeText`
  (bind _bp_playercontroller (`self.BP_PlayerController`))
  (bind _asmy_game_instance (cast `/Game/OurContent/Blueprints/MyGameInstance` (`GameplayStatics.GetGameInstance`)))
  (if (== (`/Game/OurContent/Blueprints/MyGameInstance.LoopsCount` _asmy_game_instance) 0)
    (`/Game/OurContent/Blueprints/BP_PlayerController.SetNarrativeTexts` _bp_playercontroller 2 3.75 0.0)
    (`/Game/OurContent/Blueprints/BP_PlayerController.ManagePadAMusic` _bp_playercontroller)))

(fn `UserConstructionScript`
  (`parent.UserConstructionScript`))