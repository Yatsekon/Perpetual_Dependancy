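; Room 28 level prefab that changes its decals and narrative text according to the player's loop count.
; Shortly after BeginPlay, it compares the controller's IntBoucleCount with BoucleEventLight, then BoucleEventNeeded.
; The light loop unhides all Decals descendants and the needed loop only direct children, each followed by its own delayed narrative line.
; Any other loop hides the direct decal children and both BloodLights.
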(event `self.ReceiveBeginPlay`
  (`parent.ReceiveBeginPlay`)
  (`KismetSystemLibrary.Delay` 0.1)
  (if (== (`/Game/OurContent/Blueprints/BP_PlayerController.Int_BoucleCount` (`self.BP_PlayerController`)) (`self.BoucleEventLight`))
    (for _array_element (`SceneComponent.GetChildrenComponents` (`self.Decals`) true)
      (`SceneComponent.SetHiddenInGame` _array_element false false))
    (`KismetSystemLibrary.Delay` 1.0)
    (`/Game/OurContent/Blueprints/BP_PlayerController.SetNarrativeTexts` (`self.BP_PlayerController`) 17 3.0 0.0)
    (elif (== (`/Game/OurContent/Blueprints/BP_PlayerController.Int_BoucleCount` (`self.BP_PlayerController`)) (`self.Boucle Event Needed`))
      (for _array_element_2 (`SceneComponent.GetChildrenComponents` (`self.Decals`) false)
        (`SceneComponent.SetHiddenInGame` _array_element_2 false false))
      (`KismetSystemLibrary.Delay` 1.0)
      (`/Game/OurContent/Blueprints/BP_PlayerController.SetNarrativeTexts` (`self.BP_PlayerController`) 16 2.5 0.0)
      (else
        (for _array_element_3 (`SceneComponent.GetChildrenComponents` (`self.Decals`) false)
          (`SceneComponent.SetHiddenInGame` _array_element_3 true false))
        (`SceneComponent.SetHiddenInGame` (`self.BloodLight0`) true false)
        (`SceneComponent.SetHiddenInGame` (`self.BloodLight1`) true false)))))

(fn `UserConstructionScript`
  (`parent.UserConstructionScript`))