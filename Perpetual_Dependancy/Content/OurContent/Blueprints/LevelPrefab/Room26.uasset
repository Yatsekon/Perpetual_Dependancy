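; Room26 is a level prefab room Blueprint with an event tied to a specific loop count.
; On BeginPlay it runs the parent logic, waits briefly, then compares the player controller's loop counter (IntBoucleCount) to BoucleEventNeeded.
; On a match it calls DoNotCountAntidote with the flag set and ObjEvent as the event to spawn; otherwise it destroys the ObjEvent component.
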(event `self.ReceiveBeginPlay`
  (bind _objevent (`self.ObjEvent`))
  (`parent.ReceiveBeginPlay`)
  (`KismetSystemLibrary.Delay` 0.1)
  (if (== (`/Game/OurContent/Blueprints/BP_PlayerController.Int_BoucleCount` (`self.BP_PlayerController`)) (`self.boucleEventNeeded`))
    (`self.DoNotCountAntidote` true _objevent)
    (else
      (`ActorComponent.K2_DestroyComponent` _objevent))))

(fn `UserConstructionScript`
  (`parent.UserConstructionScript`))