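; Parent room prefab for a looping level that spawns and tears down its own doors, key, checkpoint and poison or antidote spawners.
; BeginPlay uses the player controller's loop count to choose the exit point and B1 variant, then fills spawner points with random or preplaced poisons.
; It also sets music silence and jump permission, and swaps a spawner for room-specific events.
; Other events handle secret doors and material overrides on key elements.
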(event `self.ReceiveBeginPlay`
  (bind _bp_playercontroller (`self.BP_PlayerController`))
  ;[1 0.2681 0.5654] Instantiate all blueprint needed inside the map
  (`KismetSystemLibrary.Delay` 0.1)
  (bind _asbp_player_controller (cast `/Game/OurContent/Blueprints/BP_PlayerController` (`GameplayStatics.GetPlayerController` 0)))
  (bind _output_get (set `self.BP_PlayerController` _asbp_player_controller))
  (if (> (`/Game/OurContent/Blueprints/BP_PlayerController.Int_BoucleCount` _output_get) (- (`self.LoopNeeded`) 1))
    (bind _output_get_2 (set `self.RoomIsB1?` true)))
  (if (and (or (`self.B_AreMultipleDoorsSpawns`) (and _output_get_2 (`self.MultiDoorB1`))) (> (`/Game/OurContent/Blueprints/BP_PlayerController.Int_BoucleCount` _output_get) 0))
    (if (== (mod (`/Game/OurContent/Blueprints/BP_PlayerController.Int_BoucleCount` (`self.BP_PlayerController`)) 2) 1)
      (`self.SelectDoorType` (`SceneComponent.K2_GetComponentToWorld` (`self.EndPoint1`)))
      (else
        (`self.SelectDoorType` (`SceneComponent.K2_GetComponentToWorld` (`self.EndPoint0`)))))
    (else
      (`self.SelectDoorType` (`SceneComponent.K2_GetComponentToWorld` (`self.EndPoint0`)))))
  (if (`self.B_GetCheckpoint`)
    (bind _returnvalue (`|SpawnActorFromClass` "/Game/OurContent/Blueprints/BP_Checkpoint.BP_Checkpoint_C" (`SceneComponent.K2_GetComponentToWorld` (`KismetArrayLibrary.Array_Random` (`SceneComponent.GetChildrenComponents` (`self.CheckpointTransoList`) false))) "Undefined" "MultiplyWithRoot" null null))
    (set `self.BP_Checkpoint` _returnvalue))
  (if (`self.B_AreSpawnerNumberRandom`)
    (set `self.Int_SpawnerNumber` (`KismetMathLibrary.RandomInteger` 4)))
  (for (_array_element _array_index) (`SceneComponent.GetChildrenComponents` (`self.PoisonSpawnerList`) false)
    (if (and (`self.RoomIsB1?`) (`self.B SpawnerNumberChange`))
      (if (> (`self.SpawnerNumberB1`) (`self.Int_CurrentSpawner`))
        (`/Engine/EditorBlueprintResources/StandardMacros.IncrementInt` (`self.Int_CurrentSpawner`) :!label _label
          (:`  `
            (bind _returnvalue_2 (`|SpawnActorFromClass` "/Game/OurContent/Blueprints/BP_Spawner.BP_Spawner_C" (`SceneComponent.K2_GetComponentToWorld` _array_element) "Undefined" "MultiplyWithRoot" null null))
            (`KismetArrayLibrary.Array_Add` (`self.BP_Spawner`) _returnvalue_2)
            (if (`self.RoomIsB1?`)
              (if (not (`self.SpawnAntidote_B1?`))
                (if (`self.B_ArePoisonRandom`) :!label _label_2
                  (`/Game/OurContent/Blueprints/BP_Spawner.RandomPoisonSpawn` _returnvalue_2 (`self.BP_PlayerController`))
                  (elif (`self.B_ArePoisonPlacementRandom`)
                    (`self.SetRdmPoisonNewFunction`)
                    (while (`self.B_IsPoisonAlreadyUsed`)
                      (bind _b_ispoisonused (`self.SetRdmPoisonNewFunction`))
                      (set `self.B_IsPoisonAlreadyUsed` _b_ispoisonused))
                    (`/Game/OurContent/Blueprints/BP_Spawner.PoisonToSpawn` _returnvalue_2 (`self.CurrentPoison`) _bp_playercontroller)
                    (`KismetArrayLibrary.Array_Add` (`self.PoisonUsed`) (`self.CurrentPoison`))
                    (set `self.B_IsPoisonAlreadyUsed` true)
                    (else
                      (`/Game/OurContent/Blueprints/BP_Spawner.PoisonToSpawn` _returnvalue_2 (`|GetArrayItem` (`self.PoisonPreplaced`) _array_index) _bp_playercontroller))))
                (else
                  (bind _antidotespawned (`/Game/OurContent/Blueprints/BP_Spawner.SpawnAntidote` _returnvalue_2 :!label _label_3))
                  (set `self.Antidote Spawned` _antidotespawned)
                  (set `self.B_SpawnAntidote` false)))
              (elif (not (`self.B_SpawnAntidote`))
                (goto _label_2)
                (else
                  (goto _label_3)))))))
      (elif (> (`self.Int_SpawnerNumber`) (`self.Int_CurrentSpawner`))
        (goto _label))))
  (`KismetArrayLibrary.Array_Clear` (`self.PoisonUsed`))
  (if (or (`self.B_IsRoomSilence`) (`self.B_IsRoomTotalSilence`))
    (`/Game/OurContent/Blueprints/BP_PlayerController.Switch Music` (`self.BP_PlayerController`) null))
  (set `/Game/OurContent/Blueprints/BP_PlayerController.B_RoomWithoutHallu` (`self.B_IsRoomTotalSilence`) (`self.BP_PlayerController`))
  (if (and (== (`/Game/OurContent/Blueprints/BP_PlayerController.Int_BoucleCount` (`self.BP_PlayerController`)) (`self.Int_LoopToSilence`)) (`self.B_SilenceOnSpecificLoop?`))
    (`/Game/OurContent/Blueprints/BP_PlayerController.Switch Music` (`self.BP_PlayerController`) null))
  (bind _asbp_third_person_character (cast `/Game/ThirdPerson/Blueprints/BP_ThirdPersonCharacter` (`GameplayStatics.GetPlayerPawn` 0)))
  (set `/Game/ThirdPerson/Blueprints/BP_ThirdPersonCharacter.B_CanJump` (not (`self.B_ForbidPlayerJump`)) _asbp_third_person_character)
  (`self.SetupObjEvents`))

(event `SetupObjEvents`
  (bind _bp_playercontroller (`self.BP_PlayerController`))
  (bind _bp_playercontroller_2 (`self.BP_PlayerController`))
  (bind _output (`|GetArrayItem` (`self.BP_Spawner`)))
  (bind _output_2 (`|GetArrayItem` (`self.BP_Spawner`)))
  (if (== (`/Game/OurContent/Blueprints/BP_PlayerController.RoomNumber` _bp_playercontroller) (`/Game/OurContent/Blueprints/BP_PlayerController.Int_cardioscopeRoom` _bp_playercontroller))
    (`|SpawnActorFromClass` "/Game/OurContent/Blueprints/NarrativeObjects/BP_Object_Event_Cardioscope.BP_Object_Event_Cardioscope_C" (`SceneComponent.K2_GetComponentToWorld` (`self.PoisonSpawner1`)) "Undefined" "MultiplyWithRoot" null null)
    (if (!= (`KismetArrayLibrary.Array_Length` (`self.BP_Spawner`)) 0)
      (`/Game/OurContent/Blueprints/BP_Spawner.OnDestroyCustom` _output_2)
      (`self.K2_DestroyActor` _output_2)
      (`KismetArrayLibrary.Array_RemoveItem` (`self.BP_Spawner`) _output_2)
      (else
        (if (and (== (`/Game/OurContent/Blueprints/BP_PlayerController.Int_BoucleCount` _bp_playercontroller_2) (`self.boucleEventNeeded`)) (== (`/Game/OurContent/Blueprints/BP_PlayerController.RoomNumber` _bp_playercontroller_2) 18) (not (`self.B_DoNotDestroyActorOnEvent`))) :!label _label_4
          (`/Game/OurContent/Blueprints/BP_Spawner.OnDestroyCustom` _output)
          (`self.K2_DestroyActor` _output)
          (`KismetArrayLibrary.Array_RemoveItem` (`self.BP_Spawner`) _output))))
    (else
      (goto _label_4))))

(event `DestroyAllBlueprintsInside`
  (bind _secretdoor (`self.SecretDoor`))
  (bind _bp_checkpoint (`self.BP_Checkpoint`))
  (if (`self.B_IsDoorInvisible`)
    (`self.K2_DestroyActor` (`self.BP_InvisibleDoor`))
    (else
      (`self.K2_DestroyActor` (`self.BP_Door`))))
  (`/Engine/EditorBlueprintResources/StandardMacros.IsValid` _bp_checkpoint
    (:`Is Valid`
      (`self.K2_DestroyActor` _bp_checkpoint))
    (:`Is Not Valid`
      _))
  (for _array_element (`self.BP_Spawner`)
    (`/Game/OurContent/Blueprints/BP_Spawner.OnDestroyCustom` _array_element)
    (`self.K2_DestroyActor` _array_element))
  (if (!= _secretdoor null)
    (`self.K2_DestroyActor` _secretdoor)))

(event `ModifyInterestElementsMaterial`
  (params (ModifierMat :type "MaterialInterface Object Reference"))
  (bind _bp_checkpoint (`self.BP_Checkpoint`))
  (bind _modifier_mat (`self.Modifier Mat`))
  (bind _bp_key (`self.BP_Key`))
  (bind _output_get (set `self.Modifier Mat` ModifierMat))
  (`PrimitiveComponent.SetMaterial` (`/Game/OurContent/Blueprints/BP_Door.Door` (`self.BP_Door`)) 0 _output_get)
  (`/Engine/EditorBlueprintResources/StandardMacros.IsValid` _bp_checkpoint
    (:`Is Valid`
      (`/Game/OurContent/Blueprints/BP_Checkpoint.ModifyComponentsMaterial` _bp_checkpoint (`self.Modifier Mat`)))
    (:`Is Not Valid`
      _))
  (for _array_element (`self.BP_Spawner`)
    (`PrimitiveComponent.SetMaterial` (`/Game/OurContent/Blueprints/BP_Spawner.Cube` _array_element) 0 _modifier_mat)
    (bind _bp_poison (`/Game/OurContent/Blueprints/BP_Spawner.BP_Poison` _array_element))
    (`/Engine/EditorBlueprintResources/StandardMacros.IsValid` _bp_poison
      (:`Is Valid`
        (`PrimitiveComponent.SetMaterial` (`/Game/OurContent/Blueprints/PoisonList/1Bp_Poison_Glasses.Model` _bp_poison) 0 _modifier_mat))
      (:`Is Not Valid`
        (bind _bp_antidote (`/Game/OurContent/Blueprints/BP_Spawner.BP_Antidote` _array_element))
        (`/Engine/EditorBlueprintResources/StandardMacros.IsValid` _bp_antidote
          (:`Is Valid`
            (`PrimitiveComponent.SetMaterial` (`/Game/OurContent/Blueprints/BP_Antidote.Model` _bp_antidote) 0 _modifier_mat))))))
  (`/Engine/EditorBlueprintResources/StandardMacros.IsValid` _bp_key
    (:`Is Valid`
      (`PrimitiveComponent.SetMaterial` (`/Game/OurContent/Blueprints/BP_Key.Key` _bp_key) 0 _modifier_mat))))

(event `SpawnSecretDoor`
  (bind _returnvalue (`|SpawnActorFromClass` "/Game/OurContent/Blueprints/BP_Door.BP_Door_C" (`SceneComponent.K2_GetComponentToWorld` (`self.SecretDoorSpot`)) "Undefined" "MultiplyWithRoot" null null))
  (`/Game/OurContent/Blueprints/BP_Door.SetMatSecretDoor` _returnvalue)
  (set `self.SecretDoor` _returnvalue)
  (set `/Game/OurContent/Blueprints/BP_Door.B_IsSecretDoor` true _returnvalue))

(event `DestroySecretDoor`
  (`self.K2_DestroyActor` (`self.SecretDoor`)))

(event `Verify Average Time`
  (bind _bp_playercontroller (`self.BP_PlayerController`))
  (`KismetSystemLibrary.Delay` (`self.F_PlayerAverageTime`))
  (`KismetSystemLibrary.PrintString` "Average not respected")
  (if (not (`/Game/OurContent/Blueprints/BP_PlayerController.B_IsGameOverState` _bp_playercontroller))
    (`/Game/OurContent/Blueprints/BP_PlayerController.IncreaseAddiction` _bp_playercontroller -1)))

(fn `CheckEventDestroy`
  (params (Event_Comp :type "ActorComponent Object Reference"))
  (if (!= (`/Game/OurContent/Blueprints/BP_PlayerController.Int_BoucleCount` (`self.BP_PlayerController`)) (`self.boucleEventNeeded`))
    (`ActorComponent.K2_DestroyComponent` Event_Comp)))

(fn `DetermineCellCenter`
  (returns (WallCenter :type "Vector Structure"))
  (bind _origin (`KismetSystemLibrary.GetComponentBounds` (`self.Cell`)))
  (bind (_relativelocation_x _relativelocation_y _relativelocation_z) (`KismetMathLibrary.BreakVector` (`SceneComponent.RelativeLocation` (`self.CellCenterForLights`))))
  (bind (_relativelocation_x_2 _relativelocation_y_2 _relativelocation_z_2) (`KismetMathLibrary.BreakVector` (`SceneComponent.RelativeLocation` (`self.GroundCenterForLights`))))
  (return (`KismetMathLibrary.MakeVector` (.x _origin) (.y _origin) (/ (+ _relativelocation_z _relativelocation_z_2) 2.0))))

(fn `Display Event`
  (params (EventObj :type "SceneComponent Object Reference"))
  (`/Engine/EditorBlueprintResources/StandardMacros.IsValid` EventObj
    (:`Is Valid`
      (`SceneComponent.SetVisibility` EventObj true false))))

(fn `DoNotCountAntidote`
  (params (B_DoNotCountAntidote :type Boolean) (EventToSpawn :type "SceneComponent Object Reference"))
  (bind _antidote_spawned (`self.Antidote Spawned`))
  (set `/Game/OurContent/Blueprints/BP_PlayerController.B_DonotCountAntidote` B_DoNotCountAntidote (`self.BP_PlayerController`))
  (`/Engine/EditorBlueprintResources/StandardMacros.IsValid` _antidote_spawned
    (:`Is Valid`
      (set `/Game/OurContent/Blueprints/BP_Antidote.ParentRoom(Event)` self _antidote_spawned)
      (set `self.SC_ObjEventToSpawn` EventToSpawn))))

(fn `SelectDoorType`
  (params (EndPointTransform :type "Transform Structure"))
  (if (`self.B_IsDoorInvisible`)
    (bind _returnvalue (`|SpawnActorFromClass` "/Game/OurContent/Blueprints/BP_InvisibleDoor.BP_InvisibleDoor_C" EndPointTransform "Undefined" "MultiplyWithRoot" null null))
    (set `self.BP_Door` _returnvalue)
    (set `self.BP_InvisibleDoor` _returnvalue)
    (else
      (bind _returnvalue_2 (`|SpawnActorFromClass` "/Game/OurContent/Blueprints/BP_Door.BP_Door_C" EndPointTransform "Undefined" "MultiplyWithRoot" null null))
      (bind _output_get (set `self.BP_Door` _returnvalue_2))
      (if (not (not (`self.B_IsDoorLocked`)))
        (bind _asmy_game_instance (cast `/Game/OurContent/Blueprints/MyGameInstance` (`GameplayStatics.GetGameInstance`))
          (:`then`
            (if (not (== (`/Game/OurContent/Blueprints/MyGameInstance.LastCheckpoint` _asmy_game_instance) (+ (`/Game/OurContent/Blueprints/BP_PlayerController.RoomNumber` (`self.BP_PlayerController`)) 1)))
              (set `/Game/OurContent/Blueprints/BP_Door.NeedKey` true _output_get :!label _label)
              (bind _returnvalue_3 (`|SpawnActorFromClass` "/Game/OurContent/Blueprints/BP_Key.BP_Key_C" (`SceneComponent.K2_GetComponentToWorld` (`self.KeySpot`)) "Undefined" "MultiplyWithRoot" null null))
              (set `self.BP_Key` _returnvalue_3)
              (`/Game/OurContent/Blueprints/BP_PlayerController.EnableKeyFramework` (`self.BP_PlayerController`))))
          (:`CastFailed`
            (goto _label))))))
  (return))

(fn `SetRdmPoisonNewFunction`
  (returns (B_IsPoisonUsed :type Boolean))
  (bind _output_get (set `self.CurrentPoison` (`KismetArrayLibrary.Array_Random` (`self.PoisonPreplaced`))))
  (return (`KismetArrayLibrary.Array_Contains` (`self.PoisonUsed`) _output_get)))

(fn `UserConstructionScript`)