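; Room11 is a level prefab room Blueprint that fires a scripted narrative beat on a specific loop iteration.
; Shortly after BeginPlay it compares the player controller's loop count to BoucleEventNeeded.
; On a match it plays a pursuit sound, waits briefly, then sends two narrative text lines to the player controller for display.
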(event `self.ReceiveBeginPlay`
  (bind _bp_playercontroller (`self.BP_PlayerController`))
  (`parent.ReceiveBeginPlay`)
  (`KismetSystemLibrary.Delay` 0.1)
  (if (== (`/Game/OurContent/Blueprints/BP_PlayerController.Int_BoucleCount` (`self.BP_PlayerController`)) (`self.boucleEventNeeded`))
    (`GameplayStatics.PlaySound2D` "/Game/OurContent/Sounds/Hallucinations/SFX_Pursuit_01_Cue.SFX_Pursuit_01_Cue" 1.0 1.0 0.0 null null)
    (`KismetSystemLibrary.Delay` 1.5)
    (`/Game/OurContent/Blueprints/BP_PlayerController.SetNarrativeTexts` _bp_playercontroller 21 2.5 0.0)
    (`/Game/OurContent/Blueprints/BP_PlayerController.SetNarrativeTexts` _bp_playercontroller 22 2.0 0.0)))

(fn `UserConstructionScript`
  (`parent.UserConstructionScript`))