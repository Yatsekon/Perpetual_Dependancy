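; Room2 is a level prefab Blueprint that can start the player's addiction bar on a specific loop ("boucle").
; On BeginPlay it runs the parent logic, waits briefly, then compares the player controller's loop count to BoucleEventNeeded.
; If they are equal, it calls StartAddictionBar on the controller; construction only calls the parent.
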(event `self.ReceiveBeginPlay`
  (`parent.ReceiveBeginPlay`)
  (`KismetSystemLibrary.Delay` 0.1)
  (if (== (`/Game/OurContent/Blueprints/BP_PlayerController.Int_BoucleCount` (`self.BP_PlayerController`)) (`self.boucleEventNeeded`))
    (`/Game/OurContent/Blueprints/BP_PlayerController.StartAddictionBar` (`self.BP_PlayerController`))))

(fn `UserConstructionScript`
  (`parent.UserConstructionScript`))