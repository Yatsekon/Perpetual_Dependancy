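; Room12 is a level prefab Blueprint that triggers a narrative line for its room on a specific loop of the game.
; On BeginPlay it runs the parent logic, waits briefly, then reads the loop count from MyGameInstance.
; When the count equals one, it has BPPlayerController display the narrative text with its dialogue timing.
; The construction script only calls the parent, and overlap and tick are unused.
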(event `self.ReceiveBeginPlay`
  (`parent.ReceiveBeginPlay`)
  (`KismetSystemLibrary.Delay` 0.2)
  (bind _asmy_game_instance (cast `/Game/OurContent/Blueprints/MyGameInstance` (`GameplayStatics.GetGameInstance`)))
  (if (== (`/Game/OurContent/Blueprints/MyGameInstance.LoopsCount` _asmy_game_instance) 1)
    (`/Game/OurContent/Blueprints/BP_PlayerController.SetNarrativeTexts` (`self.BP_PlayerController`) 4 3.75 0.0)))

(fn `UserConstructionScript`
  (`parent.UserConstructionScript`))