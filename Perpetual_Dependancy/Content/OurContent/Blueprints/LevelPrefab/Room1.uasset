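; Room1 is a level prefab that sets up its tutorial table and reading sheet for the current loop count.
; Shortly after BeginPlay it sets the required loop to -1 if tutorials are disabled in the game instance, then runs CheckEventDestroy on both objects.
; When the player controller's loop count matches the required loop, it assigns a specific sheet number to the child-actor reading sheet.
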(event `self.ReceiveBeginPlay`
  (`parent.ReceiveBeginPlay`)
  (`KismetSystemLibrary.Delay` 0.1)
  (bind _asmy_game_instance (cast `/Game/OurContent/Blueprints/MyGameInstance` (`GameplayStatics.GetGameInstance`)))
  (if (not (`/Game/OurContent/Blueprints/MyGameInstance.AreTutoEnable` _asmy_game_instance))
    (set `self.boucleEventNeeded` -1))
  (`self.CheckEventDestroy` (`self.TutoTable`))
  (`self.CheckEventDestroy` (`self.SheetActor`))
  (if (== (`/Game/OurContent/Blueprints/BP_PlayerController.Int_BoucleCount` (`self.BP_PlayerController`)) (`self.boucleEventNeeded`))
    (bind _asbp_reading_sheet (cast `/Game/OurContent/Blueprints/Bp_ReadingSheet` (`ChildActorComponent.ChildActor` (`self.SheetActor`))))
    (set `/Game/OurContent/Blueprints/Bp_ReadingSheet.SheetNumber` 2 _asbp_reading_sheet)))

(fn `UserConstructionScript`
  (`parent.UserConstructionScript`))