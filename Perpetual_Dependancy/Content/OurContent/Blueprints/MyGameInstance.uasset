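; MyGameInstance is the game instance that holds persistent progress and option state across levels.
; ResetAllParameters clears run progress such as checkpoints, loop counts, intro flag, antidote count, used texts and addiction state.
; ResetOptions restores default tutorial, subtitle and graphics settings and clears the game-start flag.
; StartFirstInstance records whether this is the game's first instance.
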(event `ResetAllParameters`
  (set `self.LastCheckpoint` 0)
  (set `self.LoopsCount` 0)
  (set `self.LastCheckpointLoop` 0)
  (set `self.IsIntroDone` false)
  (set `self.AntidoteCount` 0)
  (`KismetArrayLibrary.Array_Clear` (`self.B Text_Used`))
  (set `self.Int_CurrentAddictionState` 0))

(event `ResetOptions`
  (set `self.AreTutoEnable` true)
  (set `self.AreSubtitleEnable` true)
  (set `self.CurrentGraphicLevel` 2)
  (set `self.GameStart` false))

(event `StartFirstInstance`
  (params (IsGameFirstInstance :type Boolean))
  (if IsGameFirstInstance
    (set `self.GameFirstInstance` true)
    (else
      (set `self.GameFirstInstance` false))))