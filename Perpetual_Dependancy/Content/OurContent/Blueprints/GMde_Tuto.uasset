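; GMde_Tuto is a tutorial game mode that sets up the player's movement and interaction tutorial state.
; On BeginPlay it caches the game instance and the third-person player character.
; When StartTuto runs on the game's first instance, it copies the instance's tutorial-enable flag into the character's move and interact flags.
; If that flag is on, it asks the player controller to create the tutorial widget.
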(event `StartTuto`
  (bind _bp_chara (`self.BP_Chara`))
  (bind _aretutoenable (`/Game/OurContent/Blueprints/MyGameInstance.AreTutoEnable` (`self.As My Game Instance`)))
  (bind _b_istutointeract (`/Game/ThirdPerson/Blueprints/BP_ThirdPersonCharacter.B_IsTutoInteract` _bp_chara))
  (if (`/Game/OurContent/Blueprints/MyGameInstance.GameFirstInstance` (`self.As My Game Instance`))
    (bind _output_get (set `/Game/ThirdPerson/Blueprints/BP_ThirdPersonCharacter.B_IsTutoMove` _aretutoenable _bp_chara))
    (for (_ _array_index) _b_istutointeract
      (`KismetArrayLibrary.Array_Set` _b_istutointeract _array_index _aretutoenable))
    (if _output_get
      (bind _asbp_player_controller (cast `/Game/OurContent/Blueprints/BP_PlayerController` (`GameplayStatics.GetPlayerController` 0)))
      (`/Game/OurContent/Blueprints/BP_PlayerController.InstanceWidgetTuto` _asbp_player_controller))))

(event `self.ReceiveBeginPlay`
  (bind _asmy_game_instance (cast `/Game/OurContent/Blueprints/MyGameInstance` (`GameplayStatics.GetGameInstance`)))
  (set `self.As My Game Instance` _asmy_game_instance)
  (bind _asbp_third_person_character (cast `/Game/ThirdPerson/Blueprints/BP_ThirdPersonCharacter` (`GameplayStatics.GetPlayerPawn` 0)))
  (set `self.BP_Chara` _asbp_third_person_character))

(fn `UserConstructionScript`)