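; Main-menu spotlight Blueprint that animates the intensity of a blue and a red light through BlueSide and RedSide events.
; A shared first-time flag makes the first call play a timeline that changes only that side's light.
; Later calls play timelines that drive both lights together, each lerping between low and high intensity, with the lerp endpoints reversed for the red side.
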(event `BlueSide`
  (if (`self.1stTime`)
    (set `self.1stTime` false)
    (bind (_direction _blueintensity) (`Timeline|1stBlueOn` :!via `PlayFromStart`)
      (:`Update`
        (`LightComponent.SetIntensity` (`self.SpotBlue`) (`KismetMathLibrary.Lerp` 0.25 5.0 _blueintensity))))
    (else
      (bind (_direction_2 _blueintensity_2 _redintensity) (`Timeline|BlueOn` :!via `PlayFromStart`)
        (:`Update`
          (`LightComponent.SetIntensity` (`self.SpotBlue`) (`KismetMathLibrary.Lerp` 0.25 5.0 _blueintensity_2))
          (`LightComponent.SetIntensity` (`self.SpotRed`) (`KismetMathLibrary.Lerp` 0.25 5.0 _redintensity)))))))

(event `RedSide`
  (if (`self.1stTime`)
    (set `self.1stTime` false)
    (bind (_direction _blueintensity _redintensity) (`Timeline|1stRedOn` :!via `PlayFromStart`)
      (:`Update`
        (`LightComponent.SetIntensity` (`self.SpotRed`) (`KismetMathLibrary.Lerp` 5.0 0.25 _redintensity))))
    (else
      (bind (_direction_2 _blueintensity_2 _redintensity_2) (`Timeline|RedOn` :!via `PlayFromStart`)
        (:`Update`
          (`LightComponent.SetIntensity` (`self.SpotBlue`) (`KismetMathLibrary.Lerp` 5.0 0.25 _blueintensity_2))
          (`LightComponent.SetIntensity` (`self.SpotRed`) (`KismetMathLibrary.Lerp` 5.0 0.25 _redintensity_2)))))))

(fn `UserConstructionScript`)