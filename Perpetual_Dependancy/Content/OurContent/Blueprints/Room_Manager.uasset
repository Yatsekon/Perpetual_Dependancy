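; Room manager that runs the game's looping room sequence, resuming from the GameInstance's last checkpoint.
; NewNextRoom destroys the current room, spawns the next RoomList entry at an index-based height, teleports the player, then updates lighting and poison.
; Passing the last room increments the loop count and restarts the list.
; It also handles music, transition sounds, room timing and a once-per-loop recursive random cardioscope room pick in later loops.
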(event `self.ReceiveBeginPlay`
  (bind _returnvalue (`GameplayStatics.GetActorOfClass` "/Game/ThirdPerson/Blueprints/BP_ThirdPersonCharacter.BP_ThirdPersonCharacter_C"))
  (set `self.Character` _returnvalue)
  (bind _returnvalue_2 (`GameplayStatics.GetActorOfClass` "/Game/OurContent/Blueprints/BP_PlayerController.BP_PlayerController_C"))
  (set `self.BP_PController` _returnvalue_2)
  (`KismetSystemLibrary.Delay` 0.1)
  (bind _asmy_game_instance (cast `/Game/OurContent/Blueprints/MyGameInstance` (`GameplayStatics.GetGameInstance`)))
  (set `self.As My Game Instance` _asmy_game_instance)
  (bind _lastcheckpoint (`/Game/OurContent/Blueprints/MyGameInstance.LastCheckpoint` _asmy_game_instance))
  (if (> _lastcheckpoint 0)
    (bind _output_get (set `self.RoomNumber` (- _lastcheckpoint 1))))
  (bind _output_get_2 (set `self.RoomCount` _output_get))
  (set `/Game/OurContent/Blueprints/BP_PlayerController.RoomNumber` _output_get_2 (`self.BP_PController`))
  (bind _output_get_3 (set `/Game/OurContent/Blueprints/BP_PlayerController.Int_BoucleCount` (`/Game/OurContent/Blueprints/MyGameInstance.LastCheckpointLoop` _asmy_game_instance) (`self.BP_PController`)))
  (set `/Game/OurContent/Blueprints/MyGameInstance.LoopsCount` _output_get_3 _asmy_game_instance)
  (`self.NewNextRoom` false))

(event `NewNextRoom`
  (params (IsLoopDoor :type Boolean))
  (bind _bp_pcontroller (`self.BP_PController`))
  (bind _bp_pcontroller_2 (`self.BP_PController`))
  (bind _bp_pcontroller_3 (`self.BP_PController`))
  (bind _bp_pcontroller_4 (`self.BP_PController`))
  (bind _timeline (`self.Timeline`))
  (bind _initangl (`self.InitAngl`))
  (bind _capsulecomponent (`Character.CapsuleComponent` (`self.Character`)))
  (bind _bp_currentroom (`/Game/OurContent/Blueprints/BP_PlayerController.BP_CurrentRoom` (`self.BP_PController`)))
  (bind _returnvalue (`KismetMathLibrary.Conv_IntToDouble` (* (`self.RoomNumber`) 500)))
  (`self.SelectMusic`)
  (if (not (`self.B_FirstInstance`))
    (`/Game/OurContent/Blueprints/BP_PlayerController.RoomTransIn` (`self.BP_PController`) IsLoopDoor)
    (`/Game/OurContent/Blueprints/LevelPrefab/BP_ParentRoom.DestroyAllBlueprintsInside` _bp_currentroom)
    (`KismetSystemLibrary.PrintString` (`KismetStringLibrary.Concat_StrStr` (`KismetStringLibrary.Concat_StrStr` "Current Time : " (`KismetStringLibrary.Conv_DoubleToString` (`self.F_PlayerTime`))) " Average Time : " (`KismetStringLibrary.Conv_DoubleToString` (`/Game/OurContent/Blueprints/LevelPrefab/BP_ParentRoom.F_PlayerAverageTime` _bp_currentroom))))
    (`self.K2_DestroyActor` _bp_currentroom)
    (if IsLoopDoor
      (bind _returnvalue_2 (`GameplayStatics.SpawnSound2D` "/Game/OurContent/Sounds/Items/Loop_Transition_Test.Loop_Transition_Test" 1.0 1.0 0.0 null))
      (`/Game/OurContent/Blueprints/BP_PlayerController.ManageSoundEffect` _bp_pcontroller _returnvalue_2)
      (`/Game/OurContent/Blueprints/BP_PlayerController.ManageAllWidget` _bp_pcontroller true)
      (`KismetSystemLibrary.Delay` 2.5)
      (else
        (`GameplayStatics.PlaySound2D` "/Game/OurContent/Sounds/Environnement/Door_-_01_Cue.Door_-_01_Cue" 1.0 1.0 0.0 null null))))
  (if (< (`self.RoomNumber`) (`KismetArrayLibrary.Array_Length` (`self.RoomList`)))
    (set `self.LastRoom` (- (`self.RoomNumber`) 1))
    (else
      (set `self.LoopPassed` true)
      (bind _result (`/Engine/EditorBlueprintResources/StandardMacros.IncrementInt` (`/Game/OurContent/Blueprints/BP_PlayerController.Int_BoucleCount` _bp_pcontroller_3))
        (:`  `
          (set `/Game/OurContent/Blueprints/MyGameInstance.LoopsCount` _result (`self.As My Game Instance`))
          (set `self.RoomNumber` 0)
          (`/Game/OurContent/Blueprints/BP_PlayerController.DisplayTextStartBoucle2+` _bp_pcontroller_3)
          (`self.ResetCardioscope`)))))
  ;[0.05098 0.05098 0.05098] Instancie la salle suivante et place le joueur dedans
  (bind _returnvalue_3 (`|SpawnActorFromClass` (`|GetArrayItem` (`self.RoomList`) (`self.RoomNumber`)) (`KismetMathLibrary.MakeTransform` (`KismetMathLibrary.MakeVector` 0.0 0.0 _returnvalue)) "Undefined" "MultiplyWithRoot" null null))
  (set `self.F_RoomHeight` _returnvalue)
  (set `/Game/OurContent/Blueprints/BP_PlayerController.BP_CurrentRoom` _returnvalue_3 _bp_pcontroller_4)
  (bind _startpoint (`/Game/OurContent/Blueprints/LevelPrefab/BP_ParentRoom.StartPoint` _returnvalue_3))
  (`Controller.SetControlRotation` _bp_pcontroller_4 (`SceneComponent.K2_GetComponentRotation` _startpoint))
  (`self.K2_SetActorTransform` (`self.Character`) (`SceneComponent.K2_GetComponentToWorld` _startpoint) false false)
  (`PrimitiveComponent.SetAllPhysicsAngularVelocityInDegrees` _capsulecomponent _initangl false)
  (`PrimitiveComponent.SetAllPhysicsLinearVelocity` _capsulecomponent _initangl false)
  (bind _wallcenter (`/Game/OurContent/Blueprints/LevelPrefab/BP_ParentRoom.DetermineCellCenter` (`/Game/OurContent/Blueprints/BP_PlayerController.BP_CurrentRoom` (`self.BP_PController`))))
  (`/Game/OurContent/Blueprints/BP_LightManager.SetupLightning` (`self.BP_LightManager`) (`KismetMathLibrary.MakeVector` (.x _wallcenter) (.y _wallcenter) (+ (.z _wallcenter) (`self.F_RoomHeight`))) (`self.RoomNumber`) (`self.LastRoom`))
  (`/Game/OurContent/Blueprints/BP_PlayerController.MajPoison` (`self.BP_PController`) (`self.RoomCount`) (`self.RoomNumber`))
  (`/Engine/EditorBlueprintResources/StandardMacros.IncrementInt` (`self.RoomNumber`)
    (:`  `
      (`/Engine/EditorBlueprintResources/StandardMacros.IncrementInt` (`self.RoomCount`)
        (:`  `
          (if (and (>= (`self.Int_CurrRdmSound`) 7) (== (`KismetMathLibrary.RandomInteger` 4) 0))
            (set `self.Int_CurrRdmSound` 0)
            (bind _returnvalue_4 (`GameplayStatics.SpawnSound2D` "/Game/OurContent/Sounds/Music/Random_Sounds.Random_Sounds" 1.0 1.0 0.0 null))
            (`/Game/OurContent/Blueprints/BP_PlayerController.ManageSoundEffect` (`self.BP_PController`) _returnvalue_4)
            (else
              (`/Engine/EditorBlueprintResources/StandardMacros.IncrementInt` (`self.Int_CurrRdmSound`)
                (:`  `
                  _))))
          (if (`self.B_FirstInstance`)
            (set `self.B_FirstInstance` false)
            (else
              (`/Game/OurContent/Blueprints/BP_PlayerController.VerifyPoisonRedistribution` _bp_pcontroller_2)
              (`/Game/OurContent/Blueprints/BP_PlayerController.RoomTransOut` _bp_pcontroller_2)
              (`/Game/OurContent/Blueprints/LevelPrefab/BP_ParentRoom.Verify Average Time` (`/Game/OurContent/Blueprints/BP_PlayerController.BP_CurrentRoom` (`self.BP_PController`)))))
          (`/Engine/EditorBlueprintResources/StandardMacros.IsValid` _timeline
            (:`Is Valid`
              (`TimelineComponent.Stop` _timeline)
              (if (> (`/Game/OurContent/Blueprints/MyGameInstance.LoopsCount` (`self.As My Game Instance`)) 2)
                (`self.DesignateTheCardioscopeRoom`)
                (bind (_direction _current_time) (`Timeline|Timeline` :!via `PlayFromStart` :!label _label)
                  (:`Update`
                    (set `self.F_PlayerTime` _current_time)))
                (else
                  (goto _label :!via `PlayFromStart`))))))))))

(event `DesignateTheCardioscopeRoom`
  (`/Engine/EditorBlueprintResources/StandardMacros.DoOnce` false :!label _label_2
    (:`Completed`
      (bind _roomdesignated (`self.Check Forbidden Rooms`))
      (set `/Game/OurContent/Blueprints/BP_PlayerController.Int_cardioscopeRoom` _roomdesignated (`self.BP_PController`)))))

(event `SelectMusic`
  (if (>= (`self.RoomNumber`) 15)
    (`/Game/OurContent/Blueprints/BP_PlayerController.Switch Music` (`self.BP_PController`) "/Game/OurContent/Sounds/Music/Amb_Opressive/Low_Drone_Loop_V2_Cue.Low_Drone_Loop_V2_Cue")
    (elif (and (< (`self.RoomNumber`) 15) (> (`/Game/OurContent/Blueprints/BP_PlayerController.Int_BoucleCount` (`self.BP_PController`)) 0))
      (`/Game/OurContent/Blueprints/BP_PlayerController.Switch Music` (`self.BP_PController`) "/Game/OurContent/Sounds/Music/Hi_Drone_A_-_01_Cue.Hi_Drone_A_-_01_Cue")
      (elif (< (`self.RoomNumber`) 15)
        (`/Game/OurContent/Blueprints/BP_PlayerController.Switch Music` (`self.BP_PController`) "/Game/OurContent/Sounds/Music/Roomtone_01_-_01_Cue.Roomtone_01_-_01_Cue")))))

(event `ResetCardioscope`
  (goto _label_2 :!via `Reset`))

(fn `Check Forbidden Rooms`
  (returns (RoomDesignated :type Integer))
  (bind _randomroom (`self.RandomRoom`))
  (set `self.RandomRoom` (`KismetMathLibrary.RandomInteger` (- (`KismetArrayLibrary.Array_Length` (`self.RoomList`)) 1)))
  (if (and (`KismetMathLibrary.Conv_IntToBool` (`KismetArrayLibrary.Array_Find` (`self.FobiddenCardioscopeRooms`) _randomroom)) (!= _randomroom (`/Game/OurContent/Blueprints/BP_PlayerController.Int_cardioscopeRoom` (`self.BP_PController`))))
    (return _randomroom)
    (else
      (`self.Check Forbidden Rooms`))))

(fn `UserConstructionScript`)