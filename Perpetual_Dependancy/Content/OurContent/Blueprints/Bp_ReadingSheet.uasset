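; Interactable reading sheet that opens the player controller's reading widget at its sheet number, locking movement and jump, switching to UI-only input and passing commentary settings.
; A looping timeline bobs its sprite icon, and Tick yaws the visible icon toward the player.
; ReadName briefly flags it readable, with DoOnce gates swapping sprite for text.
; Box overlaps fade the character's interact tutorial prompt in and out.
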(event `self.ReceiveBeginPlay`
  (set `self.PaperSprite_Origin` (`SceneComponent.K2_GetComponentLocation` (`self.PaperSprite`)))
  (`self.Float_Icon`))

(event `Float_Icon`
  (bind (_papersprite_origin_x _papersprite_origin_y _papersprite_origin_z) (`KismetMathLibrary.BreakVector` (`self.PaperSprite_Origin`)))
  (bind (_direction _newtrack_0) (`Timeline|Float_Icon_Over_Time` :!label _label)
    (:`Update`
      (`SceneComponent.K2_SetWorldLocation` (`self.PaperSprite`) (`KismetMathLibrary.MakeVector` _papersprite_origin_x _papersprite_origin_y (+ _newtrack_0 _papersprite_origin_z)) false false))
    (:`Finished`
      (`KismetSystemLibrary.Delay` 0.005)
      (goto _label :!via `PlayFromStart`))))

(event `Rotate_Showing_Icon`
  (params (Icon_Component :type "SceneComponent Object Reference") (degreeOffset :type "Float (double-precision)"))
  (bind (_returnvalue_roll _returnvalue_pitch) (`KismetMathLibrary.BreakRotator` (`SceneComponent.K2_GetComponentRotation` Icon_Component)))
  (bind (_returnvalue_roll_2 _returnvalue_pitch_2 _returnvalue_yaw) (`KismetMathLibrary.BreakRotator` (`KismetMathLibrary.FindLookAtRotation` (`SceneComponent.K2_GetComponentLocation` Icon_Component) (`self.K2_GetActorLocation` (`GameplayStatics.GetPlayerPawn` 0)))))
  (`SceneComponent.K2_SetWorldRotation` Icon_Component (`KismetMathLibrary.MakeRotator` _returnvalue_roll _returnvalue_pitch (+ _returnvalue_yaw degreeOffset)) false false))

(event `self.ReceiveTick`
  (params (DeltaSeconds :type "Float (single-precision)"))
  (if (`self.B_IsReadable`)
    (`self.Rotate_Showing_Icon` (`self.TextRender`))
    (`/Engine/EditorBlueprintResources/StandardMacros.DoOnce` false :!label _label_2
      (:`Completed`
        (`SceneComponent.SetVisibility` (`self.PaperSprite`) false false)
        (`SceneComponent.SetVisibility` (`self.TextRender`) true false)
        (goto _label_3 :!via `Reset`)))
    (else
      (`self.Rotate_Showing_Icon` (`self.PaperSprite`) 90.0)
      (`/Engine/EditorBlueprintResources/StandardMacros.DoOnce` false :!label _label_3
        (:`Completed`
          (`SceneComponent.SetVisibility` (`self.TextRender`) false false)
          (`SceneComponent.SetVisibility` (`self.PaperSprite`) true false)
          (goto _label_2 :!via `Reset`))))))

(event `/Game/OurContent/Blueprints/Other/I_Interact.PlayerInteraction`
  (params (Interactor :type "Character Object Reference"))
  (bind _as_bp_player_controller (`self.As BP Player Controller`))
  (bind _asbp_third_person_character (cast `/Game/ThirdPerson/Blueprints/BP_ThirdPersonCharacter` Interactor))
  (set `/Game/ThirdPerson/Blueprints/BP_ThirdPersonCharacter.CanMove` false _asbp_third_person_character)
  (set `/Game/ThirdPerson/Blueprints/BP_ThirdPersonCharacter.B_CanJump` false _asbp_third_person_character)
  (bind _asbp_player_controller (cast `/Game/OurContent/Blueprints/BP_PlayerController` (`GameplayStatics.GetPlayerController` 0)))
  (bind _output_get (set `self.As BP Player Controller` _asbp_player_controller))
  (set `/Game/OurContent/Blueprints/BP_PlayerController.B_isCommentaringSheet` (`self.is_MC_Commentaring`) _output_get)
  (set `/Game/OurContent/Blueprints/BP_PlayerController.Int_CommentaringNumber` (`self.Int_commentaringNumber`) _output_get)
  (bind _wg_readingsheet (`/Game/OurContent/Blueprints/BP_PlayerController.WG ReadingSheet` _asbp_player_controller))
  (set `/Game/OurContent/Widgets/WG_ReadingSheet.int_SheetNumber` (`self.SheetNumber`) _wg_readingsheet)
  (`UserWidget.AddToViewport` _wg_readingsheet 100)
  (`GameplayStatics.SpawnSound2D` "/Game/OurContent/Sounds/MenuSound/UI_Paper_01.UI_Paper_01" 1.0 1.0 0.0 null)
  (set `PlayerController.bShowMouseCursor` true _as_bp_player_controller)
  (`WidgetBlueprintLibrary.SetInputMode_UIOnlyEx` _as_bp_player_controller (`/Game/OurContent/Blueprints/BP_PlayerController.WG ReadingSheet` _as_bp_player_controller))
  (set `/Game/OurContent/Blueprints/BP_PlayerController.B_IsAddictionOn` false _as_bp_player_controller)
  (`/Game/ThirdPerson/Blueprints/BP_ThirdPersonCharacter.SetTutoInteract` _asbp_third_person_character false false true))

(event `/Game/OurContent/Blueprints/Other/I_DisplayName.Read Name`
  (set `self.B_IsReadable` true)
  (`/Engine/EditorBlueprintResources/StandardMacros.DoOnce` false :!label _label_4
    (:`Completed`
      (`SceneComponent.SetVisibility` (`self.TextRender`) true false)
      (`KismetSystemLibrary.Delay` 0.25)
      (set `self.B_IsReadable` false)
      (goto _label_4 :!via `Reset`))))

(event `self.Box.OnComponentBeginOverlap`
  (params (OverlappedComponent :type "PrimitiveComponent Object Reference") (OtherActor :type "Actor Object Reference") (OtherComp :type "PrimitiveComponent Object Reference") (OtherBodyIndex :type Integer) (bFromSweep :type Boolean) (SweepResult :type "HitResult Structure (by ref)"))
  (bind _asbp_third_person_character (cast `/Game/ThirdPerson/Blueprints/BP_ThirdPersonCharacter` OtherActor))
  (`/Game/ThirdPerson/Blueprints/BP_ThirdPersonCharacter.SetTutoInteract` _asbp_third_person_character false true false))

(event `self.Box.OnComponentEndOverlap`
  (params (OverlappedComponent :type "PrimitiveComponent Object Reference") (OtherActor :type "Actor Object Reference") (OtherComp :type "PrimitiveComponent Object Reference") (OtherBodyIndex :type Integer))
  (bind _asbp_third_person_character (cast `/Game/ThirdPerson/Blueprints/BP_ThirdPersonCharacter` OtherActor))
  (`/Game/ThirdPerson/Blueprints/BP_ThirdPersonCharacter.SetTutoInteract` _asbp_third_person_character false false false))

(fn `UserConstructionScript`)