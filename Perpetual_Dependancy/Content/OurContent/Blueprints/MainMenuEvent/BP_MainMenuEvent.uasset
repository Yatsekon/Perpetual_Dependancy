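; Main menu event actor that flashes random post-process hallucination effects, each paired with a 2D sound.
; A timer event waits a random delay, then picks a material, rerolling recent or current picks until all have played.
; The chosen material becomes a dynamic instance blendable on the PostProcess component for a set duration, then is removed and the timer restarts.
; BeginPlay is empty, so nothing here starts the cycle.
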(event `AddPostProcessEffect`
  (params (MaterialInstance :type "MaterialInstance Object Reference"))
  (bind _pp_active (`self.PP Active`))
  ;[1 0.251 0.251] PostProcessEffect
  (if (not (`KismetArrayLibrary.Array_Contains` (`self.PP MI Active`) MaterialInstance))
    (`KismetArrayLibrary.Array_Add` (`self.PP MI Active`) MaterialInstance)
    (bind _returnvalue (`KismetMaterialLibrary.CreateDynamicMaterialInstance` MaterialInstance))
    (`KismetArrayLibrary.Array_Add` (`self.PP MID Active`) _returnvalue)
    (`KismetArrayLibrary.Array_Add` _pp_active (make `WeightedBlendable` 1.0 _returnvalue))
    (set `PostProcessComponent.Settings` (make `PostProcessSettings` :`WeightedBlendables` (make `WeightedBlendables` _pp_active)) (`self.PostProcess`))))

(event `RemovePostProcessEffect`
  (params (MaterialInstance :type "MaterialInstance Object Reference"))
  (bind _pp_active (`self.PP Active`))
  (bind _returnvalue (`KismetArrayLibrary.Array_Find` (`self.PP MI Active`) MaterialInstance))
  ;[1 0.251 0.251] PostProcessEffect
  (if (not (== _returnvalue -1))
    (`KismetArrayLibrary.Array_RemoveItem` _pp_active (make `WeightedBlendable` 1.0 (`|GetArrayItem` (`self.PP MID Active`) _returnvalue)))
    (set `PostProcessComponent.Settings` (make `PostProcessSettings` :`WeightedBlendables` (make `WeightedBlendables` _pp_active)) (`self.PostProcess`))
    (`KismetArrayLibrary.Array_Remove` (`self.PP MID Active`) _returnvalue)
    (`KismetArrayLibrary.Array_RemoveItem` (`self.PP MI Active`) MaterialInstance)))

(event `TimerRdm_Post_Process_Event`
  (bind (_v2_clamprandom_x _v2_clamprandom_y) (`KismetMathLibrary.BreakVector2D` (`self.V2_ClampRandom`)))
  (bind _output_get (set `self.F_RandomEventProc` (`KismetMathLibrary.RandomFloatInRange` _v2_clamprandom_x _v2_clamprandom_y)))
  (`KismetSystemLibrary.Delay` _output_get)
  (`self.InstancePostProcessEvent`))

(event `self.ReceiveBeginPlay`)

(event `InstancePostProcessEvent`
  (bind _mi_currmaterialinstance (`self.MI_CurrMaterialInstance`))
  (`self.ResetEvents`)
  (if (not (!= _mi_currmaterialinstance null))
    (`self.RemovePostProcessEffect` _mi_currmaterialinstance))
  (bind _isvalide (`self.RdmPostProcess` :!label _label))
  (if _isvalide
    (bind _output_get (set `self.MI_CurrMaterialInstance` (`self.MI_RdmMaterialInstance`)))
    (set `self.Int_HalluSound` (`KismetArrayLibrary.Array_Find` (`self.MI_AllMaterialInstance`) _output_get))
    (`self.Select_Hallu_Sound`)
    (`self.AddPostProcessEffect` _output_get)
    (`KismetArrayLibrary.Array_Add` (`self.MI_ArrayLastMatsInstance`) _output_get)
    (`KismetSystemLibrary.Delay` (`self.F_PP_Duration`))
    (`self.RemovePostProcessEffect` (`self.MI_CurrMaterialInstance`))
    (`self.TimerRdm_Post_Process_Event`)
    (else
      (goto _label))))

(event `Select_Hallu_Sound`
  (switch `int` (`self.Int_HalluSound`)
    (:`Default`
      (`GameplayStatics.PlaySound2D` "/Game/OurContent/Sounds/MenuSound/Menu_FX_04_01_Cue.Menu_FX_04_01_Cue" 1.0 1.0 0.0 null null :!label _label_2))
    (:`0`
      (goto _label_2))
    (:`1`
      (`GameplayStatics.PlaySound2D` "/Game/OurContent/Sounds/MenuSound/Menu_FX_02_01_Cue.Menu_FX_02_01_Cue" 1.0 1.0 0.0 null null))
    (:`2`
      (`GameplayStatics.PlaySound2D` "/Game/OurContent/Sounds/MenuSound/Menu_FX_01_01_Cue.Menu_FX_01_01_Cue" 1.0 1.0 0.0 null null))))

(event `ResetEvents`
  (if (== (`KismetArrayLibrary.Array_Length` (`self.MI_ArrayLastMatsInstance`)) (`KismetArrayLibrary.Array_Length` (`self.MI_AllMaterialInstance`)))
    (`KismetArrayLibrary.Array_Clear` (`self.MI_ArrayLastMatsInstance`))))

(fn `RdmPostProcess`
  (returns (IsValide :type Boolean))
  (bind _output_get (set `self.MI_RdmMaterialInstance` (`KismetArrayLibrary.Array_Random` (`self.MI_AllMaterialInstance`))))
  (return (and (== (`KismetArrayLibrary.Array_Find` (`self.MI_ArrayLastMatsInstance`) _output_get) -1) (!= (`self.MI_CurrMaterialInstance`) _output_get))))

(fn `UserConstructionScript`)